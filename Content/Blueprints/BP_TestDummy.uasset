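; BP_TestDummy is a sprite-based test character that automatically fires projectiles on a looping timer.
; BeginPlay caches capsule scale and starts the timer, which spawns BP_BaseProjectile at the Scene component's transform.
; Tick flips the sprite by X velocity when a controller exists, while landing restarts sprite playback and runs a timeline-driven capsule squash.
; Projectile RPC events are stubs, and the SetupInputMapping function is never called here.
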(event Custom|UpdateSpriteFlipping
  (bind _sprite (Variables|Default|GetSprite))
  ;[1 1 1] Flip Sprite Based on x velocity
  (Utilities|IsValid (Pawn|GetController)
    (:Is%20Valid
      (Math|Float|CompareFloat (.X (Class|KismetMathLibrary|BreakVector3f (Variables|/Script/Engine.MovementComponent|GetVelocity (Variables|Character|GetCharacterMovement)))) 0.0
        (:>
          (Transformation|SetRelativeRotation _sprite (Math|Rotator|MakeRotator 0.0 0.0 0.0) false false))
        (:<
          (Transformation|SetRelativeRotation _sprite (Math|Rotator|MakeRotator 0.0 0.0 -1.8e+02) false false))))))

(event Custom|LandSquish
  (bind _basescale (Variables|Default|GetBaseScale))
  ;[1 1 1] Squash N Stretch
  (bind _alpha (Timeline|Timeline_0 PlayFromStart)
    (:Update
      (Transformation|SetRelativeScale3D (Variables|Collision|GetCapsuleComponent) (Math|Vector|Lerp(Vector) _basescale (* _basescale (Variables|Default|GetLandSquishFactor)) _alpha)))))

(event Custom|RPC_FireProjectile)

(event Custom|RPC_Server_FireProjectile
  (CallFunction|RPCFireProjectile))

(event Custom|DummyShoot
  (bind _scene (Variables|Default|GetScene))
  (bind _returnvalue (Transformation|GetWorldTransform _scene))
  (bind (_location _rotation) (Math|Transform|BreakTransform _returnvalue))
  ;[1 1 1] Shooting
  (Game|SpawnActorfromClass "/Game/Blueprints/BP_BaseProjectile.BP_BaseProjectile_C" (Math|Transform|MakeTransform _location _rotation) "AdjustIfPossibleButAlwaysSpawn" 0 0))

(event EventBeginPlay
  ;[0.05098 0.05098 0.05098] Start
  (Variables|Default|SetBaseScale (Variables|/Script/Engine.SceneComponent|GetRelativeScale3D (Variables|Collision|GetCapsuleComponent)))
  (Utilities|Time|SetTimerbyEvent (delegate Custom|DummyShoot) 1.0 true))

(event EventTick
  (params (DeltaSeconds :type Float%20%28single-precision%29))
  ;[1 1 1] Update
  (CallFunction|UpdateSpriteFlipping))

(event EventOnLanded
  (params (Hit :type Hit%20Result%20Structure%20%28by%20ref%29))
  (bind _sprite (Variables|Default|GetSprite))
  ;[1 1 1] Landing
  (Components|Timeline|SetLooping _sprite true)
  (Audio|Components|Audio|Play _sprite)
  (CallFunction|LandSquish))

(fn ConstructionScript)

(fn SetupInputMapping
  (bind _asplayer_controller (Utilities|Casting|CastToPlayerController (Pawn|GetController)))
  (Utilities|IsValid (PlayerController|LocalPlayerSubsystems|GetEnhancedInputLocalPlayerSubsystem _asplayer_controller)
    (:Is%20Valid
      (Input|AddMappingContext (PlayerController|LocalPlayerSubsystems|GetEnhancedInputLocalPlayerSubsystem _asplayer_controller) "/Game/Input/IMC_Default.IMC_Default" 0 "(bIgnoreAllPressedKeysUntilRelease=True,bForceImmediately=False)"))))