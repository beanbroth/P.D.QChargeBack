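; Base 2D flipbook player character with Enhanced Input movement and jumping, mouse-aimed shooting through ACShoot, and a slash that deflects projectiles.
; Tick drives animation, sprite flipping and gun aim unless an override animation or hit stun is active.
; The slash turns overlapping projectiles toward the aim, switches their collision channel and teleports the player toward them.
; Bullet hits cause knockback, flashing and input lock; timelines add squash-and-stretch.
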(event OnComponentBeginOverlap(ChargeBackRange)
  (params (OverlappedComponent :type Primitive%20Component%20Object%20Reference) (OtherActor :type Actor%20Object%20Reference) (OtherComp :type Primitive%20Component%20Object%20Reference) (OtherBodyIndex :type Integer) (bFromSweep :type Boolean) (SweepResult :type Hit%20Result%20Structure%20%28by%20ref%29))
  (if (!= (Collision|GetCollisionObjectType OtherComp) (Math|Conversions|ToInteger(Byte) (Utilities|Enum|LiteralenumECollisionChannel "ECC_GameTraceChannel1")))
    _))

(event Custom|UpdateGroundAnimation
  ;[0.7344 1 0] Ground Animaiton Controller (runnin/idle)
  (if (AI|Components|NavMovement|IsMovingonGround (Variables|Character|GetCharacterMovement))
    (Sprite|SetFlipbook (Variables|Default|GetSprite) (select (> (Math|Float|Absolute(Float) (.X (Class|KismetMathLibrary|BreakVector3f (Variables|/Script/Engine.MovementComponent|GetVelocity (Variables|Character|GetCharacterMovement))))) 0.0) "/Game/2DCharacterSprites/YH_Cowboy_Walk1.YH_Cowboy_Walk1" "/Game/2DCharacterSprites/Idle.Idle"))
    (else
      (Sprite|SetFlipbook (Variables|Default|GetSprite) "/Game/2DCharacterSprites/Jump.Jump"))))

(event Custom|UpdateSpriteFlipping
  (bind _sprite (Variables|Default|GetSprite))
  ;[0.07812 0 1] Flip Sprite Based on x velocity
  (Utilities|IsValid (Pawn|GetController)
    (:Is%20Valid
      (Math|Float|CompareFloat (.X (Class|KismetMathLibrary|BreakVector3f (Variables|/Script/Engine.MovementComponent|GetVelocity (Variables|Character|GetCharacterMovement)))) 0.0
        (:>
          (Transformation|SetRelativeRotation _sprite (Math|Rotator|MakeRotator 0.0 0.0 0.0) false false))
        (:==
          (Transformation|SetRelativeRotation _sprite (Math|Rotator|MakeRotator 0.0 0.0 (* 9e+01 (+ (Math|Float|Sign(Float) (.X (Class|KismetMathLibrary|BreakVector3f (Math|Vector|ProjectVectorontoPlane (.WorldDirection (Game|Player|ConvertMouseLocationToWorldSpace (Game|GetPlayerController 0))) (Math|Vector|GetForwardVector (Variables|Default|GetCamera)))))) -1.0))) false false))
        (:<
          (Transformation|SetRelativeRotation _sprite (Math|Rotator|MakeRotator 0.0 0.0 -1.8e+02) false false))))))

(event Custom|PlayWalkingSounds
  ;[0.125 0 1] Horizontal Movement
  (if (AI|Components|NavMovement|IsMovingonGround (Variables|Character|GetCharacterMovement))
    (Audio|PlaySoundatLocation "/Game/Audio/Footstep.Footstep" (Transformation|GetActorLocation) "0, 0, 0" 1.0 1.0 0.0 0 0 0 0)))

(event Custom|LandSquish
  (bind _basescale (Variables|Default|GetBaseScale))
  ;[1 0.4453 0] Squash N Stretch
  (bind _alpha (Timeline|Timeline_0 PlayFromStart)
    (:Update
      (Transformation|SetRelativeScale3D (Variables|Collision|GetCapsuleComponent) (Math|Vector|Lerp(Vector) _basescale (* _basescale (Variables|Default|GetLandSquishFactor)) _alpha)))))

(event Custom|JumpSqueeze
  (bind _basescale (Variables|Default|GetBaseScale))
  ;[1 0.4453 0] Squash N Stretch
  (bind _alpha (Timeline|Timeline PlayFromStart)
    (:Update
      (Transformation|SetRelativeScale3D (Variables|Collision|GetCapsuleComponent) (Math|Vector|Lerp(Vector) _basescale (* _basescale (Variables|Default|GetJumpSqueezeFactor)) _alpha)))))

(event Custom|RPC_FireProjectile)

(event Custom|RotateGun
  ;[0 1 0.9531] Rotate Gun
  (Transformation|SetRelativeRotation (Variables|Default|GetScene) (Math|Rotator|MakeRotfromX (Math|Vector|ProjectVectorontoPlane (.WorldDirection (Game|Player|ConvertMouseLocationToWorldSpace (Game|GetPlayerController 0))) (Math|Vector|GetForwardVector (Variables|Default|GetCamera)))) false false))

(event Custom|RPC_Server_FireProjectile
  (CallFunction|RPCFireProjectile))

(event Custom|FlashSprite
  (params (NumFlashes :type Integer) (FlashDuration :type Float%20%28double-precision%29) (FlashFrequency :type Float%20%28double-precision%29) (Color :type Color%20Structure))
  (bind _sprite (Variables|Default|GetSprite))
  ;[0.7109 0 1] Flashing
  (if (< (Variables|Default|GetFlashCount) NumFlashes) :!label _label
    (Math|Integer|IncrementInt (Variables|Default|GetFlashCount)
      (:%20%20
        (Sprite|SetSpriteColor _sprite (Math|Conversions|ToLinearColor(Color) Color))
        (Utilities|FlowControl|Delay FlashDuration)
        (Sprite|SetSpriteColor _sprite (Variables|Default|GetBaseColor))
        (Utilities|FlowControl|Delay FlashFrequency)
        (goto _label)))
    (else
      (Variables|Default|SetFlashCount 0))))

(event Custom|PlayOverrideAnimation
  (params (NewFlipbook :type Paper%20Flipbook%20Object%20Reference))
  (bind _sprite (Variables|Default|GetSprite))
  ;[0.07812 0 1] Flip Sprite Based on x velocity
  (Variables|Default|SetAnimationOverride true)
  (Components|Timeline|SetLooping _sprite false)
  (Sprite|SetFlipbook _sprite NewFlipbook)
  (Utilities|FlowControl|Delay (Class|PaperFlipbook|GetTotalDuration NewFlipbook))
  (Utilities|FlowControl|DelayUntilNextTick)
  (Components|Timeline|SetLooping (Variables|Default|GetSprite) true)
  (Variables|Default|SetAnimationOverride false))

(event Input|EnhancedActionEvents|EnhancedInputActionIA_Jump
  (params (ActionValue :type Boolean) (ElapsedSeconds :type Float%20%28double-precision%29) (TriggeredSeconds :type Float%20%28double-precision%29) (InputAction :type Input%20Action%20Object%20Reference :default "/Game/Input/Actions/IA_Jump.IA_Jump"))
  ;[0.7812 1 0] Jump Controller
  (:Triggered
    (Character|Jump)
    (if (AI|Components|NavMovement|IsMovingonGround (Variables|Character|GetCharacterMovement))
      (CallFunction|JumpSqueeze)))
  (:Started
    (Audio|PlaySoundatLocation "/Game/Audio/Jump.Jump" (Transformation|GetActorLocation) "0, 0, 0" 1.0 1.0 0.0 0 0 0 0))
  (:Completed
    (Character|StopJumping)))

(event Input|EnhancedActionEvents|EnhancedInputActionIA_Move
  (params (ActionValue :type Vector%202D%20Structure) (ElapsedSeconds :type Float%20%28double-precision%29) (TriggeredSeconds :type Float%20%28double-precision%29) (InputAction :type Input%20Action%20Object%20Reference :default "/Game/Input/Actions/IA_Move.IA_Move"))
  ;[0.125 0 1] Horizontal Movement
  (:Triggered
    (Pawn|Input|AddMovementInput "1.000000,0.000000,0.000000" (.x ActionValue) false)
    (Development|PrintString "Moving"))
  (:Started
    (bind _returnvalue (Utilities|Time|SetTimerbyEvent (delegate Custom|PlayWalkingSounds) 0.25 true))
    (if (AI|Components|NavMovement|IsMovingonGround (Variables|Character|GetCharacterMovement))
      (Audio|PlaySoundatLocation "/Game/Audio/Footstep.Footstep" "0, 0, 0" "0, 0, 0" 1.0 1.0 0.0 0 0 0 0)))
  (:Canceled
    (Utilities|Time|ClearandInvalidateTimerbyHandle _returnvalue :!label _label))
  (:Completed
    (goto _label)))

(event Collision|EventHit
  (params (MyComp :type Primitive%20Component%20Object%20Reference) (Other :type Actor%20Object%20Reference) (OtherComp :type Primitive%20Component%20Object%20Reference) (bSelfMoved :type Boolean) (HitLocation :type Vector :default "0, 0, 0") (HitNormal :type Vector :default "0, 0, 0") (NormalImpulse :type Vector :default "0, 0, 0") (Hit :type Hit%20Result%20Structure%20%28by%20ref%29))
  (bind _returnvalue (Game|GetPlayerController 0))
  ;[0.2422 0 1] GetHit
  (if (Actor|ActorHasTag Other "Bullet")
    (Sprite|SetFlipbook (Variables|Default|GetSprite) "/Game/2DCharacterSprites/Jump.Jump")
    (Variables|Default|SetAnimationOverride true)
    (Character|LaunchCharacter "1000.000000,0.000000,1000.000000" false false)
    (CallFunction|FlashSprite 3 0.1 0.1 (Math|Color|MakeColor 0 0 255 255))
    (Audio|PlaySoundatLocation "/Game/Audio/Hurt.Hurt" (Transformation|GetActorLocation) "0, 0, 0" 1.0 1.0 0.0 0 0 0 0)
    (Input|SetIgnoreMoveInput _returnvalue true)
    (Utilities|FlowControl|Delay (Variables|Default|GetHitStunDurration))
    (Input|SetIgnoreMoveInput _returnvalue false)
    (Input|ResetIgnoreMoveInput _returnvalue)
    (Variables|Default|SetAnimationOverride false)))

(event EventBeginPlay
  ;[0.05098 0.05098 0.05098] Start
  (CallFunction|SetupInputMapping)
  (Variables|Default|SetBaseScale (Variables|/Script/Engine.SceneComponent|GetRelativeScale3D (Variables|Collision|GetCapsuleComponent)))
  (Variables|/Script/Engine.PlayerController|SetbShowMouseCursor (Game|GetPlayerController 0) true))

(event EventTick
  (params (DeltaSeconds :type Float%20%28single-precision%29))
  ;[1 0.1172 0] Update
  (if (not (Variables|Default|GetAnimationOverride))
    (CallFunction|UpdateGroundAnimation)
    (CallFunction|UpdateSpriteFlipping)
    (CallFunction|RotateGun)))

(event EventOnLanded
  (params (Hit :type Hit%20Result%20Structure%20%28by%20ref%29))
  (bind _sprite (Variables|Default|GetSprite))
  ;[0.8984 1 0] Landing
  (Audio|PlaySoundatLocation "/Game/Audio/Landing.Landing" (Transformation|GetActorLocation) "0, 0, 0" 1.0 1.0 0.0 0 0 0 0)
  (Components|Timeline|SetLooping _sprite true)
  (Audio|Components|Audio|Play _sprite)
  (CallFunction|LandSquish))

(event Input|MouseEvents|RightMouseButton
  (params (Key :type Key%20Structure :default "None"))
  (:Pressed
    (CallFunction|PlayOverrideAnimation "/Game/2DCharacterSprites/YH_Cowboy_VertSlash.YH_Cowboy_VertSlash")
    (CallFunction|LandSquish)
    (CallFunction|ChargeBack)))

(event Input|MouseEvents|LeftMouseButton
  (params (Key :type Key%20Structure :default "None"))
  ;[0.3359 0 1] Shooting
  (:Pressed
    (Default|DefaultShot (Variables|Default|GetAC_Shoot) (Transformation|GetWorldTransform (Variables|Default|GetBulletSpawn)))))

(event Input|KeyboardEvents|C
  (params (Key :type Key%20Structure :default "None"))
  (:Pressed
    (CallFunction|PlayOverrideAnimation "/Game/2DCharacterSprites/YH_Cowboy_VertSlash.YH_Cowboy_VertSlash")
    (CallFunction|LandSquish)
    (CallFunction|ChargeBack)))

(fn ConstructionScript)

(fn SetupInputMapping
  (bind _asplayer_controller (Utilities|Casting|CastToPlayerController (Pawn|GetController)))
  (Utilities|IsValid (PlayerController|LocalPlayerSubsystems|GetEnhancedInputLocalPlayerSubsystem _asplayer_controller)
    (:Is%20Valid
      (Input|AddMappingContext (PlayerController|LocalPlayerSubsystems|GetEnhancedInputLocalPlayerSubsystem _asplayer_controller) "/Game/Input/IMC_Default.IMC_Default" 0 "(bIgnoreAllPressedKeysUntilRelease=True,bForceImmediately=False)"))))

(fn ChargeBack
  (bind _returnvalue (Transformation|GetActorLocation))
  (bind _returnvalue_2 (Transformation|GetActorLocation))
  (bind (_outactors _returnvalue_3) (Collision|ComponentOverlapActors (Variables|Default|GetChargeBackRange) (Transformation|GetWorldTransform (Variables|Default|GetChargeBackRange)) (Utilities|Array|MakeArray "ObjectTypeQuery8") "/Game/Blueprints/BP_BaseProjectile.BP_BaseProjectile_C"))
  (if _returnvalue_3
    (Audio|PlaySoundatLocation "/Game/Audio/ChargeBack.ChargeBack" _returnvalue "0, 0, 0" 1.0 1.0 0.0 0 0 0 0)
    (for _array_element _outactors
      (Transformation|SetActorRotation _array_element (Variables|/Script/Engine.SceneComponent|GetRelativeRotation (Variables|Default|GetScene)))
      (Collision|SetCollisionObjectType (Actor|GetComponentbyClass _array_element "/Script/Engine.SphereComponent") "ECC_GameTraceChannel1")
      (Transformation|Teleport (+ _returnvalue_2 (* (Math|Vector|Normalize (- (Transformation|GetActorLocation _array_element) _returnvalue_2)) 75.0)) (Transformation|GetActorRotation))
      (CallFunction|FlashSprite 1 0.1 0.0 (Math|Color|MakeColor 0 255 0 255)))
    (else
      (Audio|PlaySoundatLocation "/Game/Audio/Woosh.Woosh" _returnvalue "0, 0, 0" 1.0 1.0 0.0 0 0 0 0))))