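; Player character for a 2D side-scroller that runs along X, jumps, aims a gun with the mouse and fires projectiles.
; Enhanced Input drives movement, while Tick switches idle/run flipbooks and flips the sprite by velocity.
; The gun arm rotates from the negated, deprojected mouse direction projected onto the camera plane, and left click spawns projectiles at an arrow component.
; Timelines squash and stretch the capsule on jump and landing.
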(event Custom|UpdateGroundAnimation
  ;[1 1 1] Ground Animaiton Controller (runnin/idle)
  (if (AI|Components|NavMovement|IsMovingonGround (Variables|Character|GetCharacterMovement))
    (Sprite|SetFlipbook (Variables|Default|GetSprite) (select (> (Math|Float|Absolute(Float) (.X (Class|KismetMathLibrary|BreakVector3f (Variables|/Script/Engine.MovementComponent|GetVelocity (Variables|Character|GetCharacterMovement))))) 0.0) "/Game/2DCharacterSprites/Run.Run" "/Game/2DCharacterSprites/Idle.Idle"))))

(event Custom|UpdateSpriteFlipping
  (bind _sprite (Variables|Default|GetSprite))
  ;[1 1 1] Flip Sprite Based on x velocity
  (Utilities|IsValid (Pawn|GetController)
    (:Is%20Valid
      (Math|Float|CompareFloat (.X (Class|KismetMathLibrary|BreakVector3f (Variables|/Script/Engine.MovementComponent|GetVelocity (Variables|Character|GetCharacterMovement)))) 0.0
        (:>
          (Transformation|SetRelativeRotation _sprite (Math|Rotator|MakeRotator 0.0 0.0 0.0) false false))
        (:<
          (Transformation|SetRelativeRotation _sprite (Math|Rotator|MakeRotator 0.0 0.0 -1.8e+02) false false))))))

(event Custom|LandSquish
  (bind _basescale (Variables|Default|GetBaseScale))
  ;[1 1 1] Squash N Stretch
  (bind _alpha (Timeline|Timeline_0 PlayFromStart)
    (:Update
      (Transformation|SetRelativeScale3D (Variables|Collision|GetCapsuleComponent) (Math|Vector|Lerp(Vector) _basescale (* _basescale (Variables|Default|GetLandSquishFactor)) _alpha)))))

(event Custom|JumpSqueeze
  (bind _basescale (Variables|Default|GetBaseScale))
  ;[1 1 1] Squash N Stretch
  (bind _alpha (Timeline|Timeline PlayFromStart)
    (:Update
      (Transformation|SetRelativeScale3D (Variables|Collision|GetCapsuleComponent) (Math|Vector|Lerp(Vector) _basescale (* _basescale (Variables|Default|GetJumpSqueezeFactor)) _alpha)))))

(event Custom|RotateGun
  ;[1 1 1] Rotate Gun
  (Transformation|SetRelativeRotation (Variables|Default|GetGun%20Arm) (Math|Rotator|MakeRotfromX (Math|Vector|ProjectVectorontoPlane (Math|Vector|NegateVector (.WorldDirection (Game|Player|ConvertMouseLocationToWorldSpace (Game|GetPlayerController 0)))) (Math|Vector|GetForwardVector (Variables|Default|GetCamera)))) false false))

(event Input|EnhancedActionEvents|EnhancedInputActionIA_Jump
  (params (ActionValue :type Boolean) (ElapsedSeconds :type Float%20%28double-precision%29) (TriggeredSeconds :type Float%20%28double-precision%29) (InputAction :type Input%20Action%20Object%20Reference :default "/Game/ThirdPerson/Input/Actions/IA_Jump.IA_Jump"))
  (bind _sprite (Variables|Default|GetSprite))
  ;[1 1 1] Jump Controller
  (:Triggered
    (Character|Jump)
    (Components|Timeline|SetLooping _sprite false)
    (Sprite|SetFlipbook _sprite "/Game/2DCharacterSprites/Jump.Jump")
    (if (AI|Components|NavMovement|IsMovingonGround (Variables|Character|GetCharacterMovement))
      (CallFunction|JumpSqueeze)))
  (:Completed
    (Character|StopJumping)))

(event Input|EnhancedActionEvents|EnhancedInputActionIA_Move
  (params (ActionValue :type Vector%202D%20Structure) (ElapsedSeconds :type Float%20%28double-precision%29) (TriggeredSeconds :type Float%20%28double-precision%29) (InputAction :type Input%20Action%20Object%20Reference :default "/Game/ThirdPerson/Input/Actions/IA_Move.IA_Move"))
  ;[1 1 1] Horizontal Movement
  (:Triggered
    (Pawn|Input|AddMovementInput "1.000000,0.000000,0.000000" (.x ActionValue) false)))

(event EventBeginPlay
  ;[0.05098 0.05098 0.05098] Start
  (CallFunction|SetupInputMapping)
  (Variables|Default|SetBaseScale (Variables|/Script/Engine.SceneComponent|GetRelativeScale3D (Variables|Collision|GetCapsuleComponent)))
  (Variables|/Script/Engine.PlayerController|SetbShowMouseCursor (Game|GetPlayerController 0) true))

(event EventTick
  (params (DeltaSeconds :type Float%20%28single-precision%29))
  ;[1 1 1] Update
  (CallFunction|UpdateGroundAnimation)
  (CallFunction|UpdateSpriteFlipping)
  (CallFunction|RotateGun))

(event EventOnLanded
  (params (Hit :type Hit%20Result%20Structure%20%28by%20ref%29))
  (bind _sprite (Variables|Default|GetSprite))
  ;[1 1 1] Landing
  (Development|PrintString "Landed")
  (Components|Timeline|SetLooping _sprite true)
  (Audio|Components|Audio|Play _sprite)
  (CallFunction|LandSquish))

(event Input|MouseEvents|LeftMouseButton
  (params (Key :type Key%20Structure :default "None"))
  (bind _arrow1 (Variables|Default|GetArrow1))
  (bind _returnvalue (Transformation|GetWorldTransform _arrow1))
  (bind (_location _rotation) (Math|Transform|BreakTransform _returnvalue))
  (:Pressed
    (Game|SpawnActorfromClass "/Game/Blueprints/Projectile.Projectile_C" (Math|Transform|MakeTransform _location _rotation) "AlwaysSpawn" 0 0)))

(fn ConstructionScript)

(fn SetupInputMapping
  (bind _asplayer_controller (Utilities|Casting|CastToPlayerController (Pawn|GetController)))
  (Utilities|IsValid (PlayerController|LocalPlayerSubsystems|GetEnhancedInputLocalPlayerSubsystem _asplayer_controller)
    (:Is%20Valid
      (Input|AddMappingContext (PlayerController|LocalPlayerSubsystems|GetEnhancedInputLocalPlayerSubsystem _asplayer_controller) "/Game/ThirdPerson/Input/IMC_Default.IMC_Default" 0 "(bIgnoreAllPressedKeysUntilRelease=True,bForceImmediately=False)"))))