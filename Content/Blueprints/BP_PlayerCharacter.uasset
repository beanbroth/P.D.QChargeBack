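; Player character for a 2D side-scrolling cowboy shooter, with Enhanced Input movement and jumping, flipbook animation and capsule squash-and-stretch.
; Tick updates animation, sprite facing and mouse-driven gun aim, while left click fires projectiles that inherit shooter velocity.
; Right click or C plays a slash, sets an animation override that is never cleared, and rotates nearby projectiles toward the aim.
; Bullet hits cause knockback, red flashing and input stun; RPC events are unfinished.
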(event OnComponentBeginOverlap(ChargeBackRange)
  (params (OverlappedComponent :type Primitive%20Component%20Object%20Reference) (OtherActor :type Actor%20Object%20Reference) (OtherComp :type Primitive%20Component%20Object%20Reference) (OtherBodyIndex :type Integer) (bFromSweep :type Boolean) (SweepResult :type Hit%20Result%20Structure%20%28by%20ref%29))
  (if (!= (Collision|GetCollisionObjectType OtherComp) (Math|Conversions|ToInteger(Byte) (Utilities|Enum|LiteralenumECollisionChannel "ECC_GameTraceChannel1")))
    _))

(event Custom|UpdateGroundAnimation
  ;[1 1 1] Ground Animaiton Controller (runnin/idle)
  (if (AI|Components|NavMovement|IsMovingonGround (Variables|Character|GetCharacterMovement))
    (Sprite|SetFlipbook (Variables|Default|GetSprite) (select (> (Math|Float|Absolute(Float) (.X (Class|KismetMathLibrary|BreakVector3f (Variables|/Script/Engine.MovementComponent|GetVelocity (Variables|Character|GetCharacterMovement))))) 0.0) "/Game/2DCharacterSprites/YH_Cowboy_Walk1.YH_Cowboy_Walk1" "/Game/2DCharacterSprites/Idle.Idle"))))

(event Custom|UpdateSpriteFlipping
  (bind _sprite (Variables|Default|GetSprite))
  ;[1 1 1] Flip Sprite Based on x velocity
  (Utilities|IsValid (Pawn|GetController)
    (:Is%20Valid
      (Math|Float|CompareFloat (.X (Class|KismetMathLibrary|BreakVector3f (Variables|/Script/Engine.MovementComponent|GetVelocity (Variables|Character|GetCharacterMovement)))) 0.0
        (:>
          (Transformation|SetRelativeRotation _sprite (Math|Rotator|MakeRotator 0.0 0.0 0.0) false false))
        (:<
          (Transformation|SetRelativeRotation _sprite (Math|Rotator|MakeRotator 0.0 0.0 -1.8e+02) false false))))))

(event Custom|LandSquish
  (bind _basescale (Variables|Default|GetBaseScale))
  ;[1 1 1] Squash N Stretch
  (bind _alpha (Timeline|Timeline_0 PlayFromStart)
    (:Update
      (Transformation|SetRelativeScale3D (Variables|Collision|GetCapsuleComponent) (Math|Vector|Lerp(Vector) _basescale (* _basescale (Variables|Default|GetLandSquishFactor)) _alpha)))))

(event Custom|JumpSqueeze
  (bind _basescale (Variables|Default|GetBaseScale))
  ;[1 1 1] Squash N Stretch
  (bind _alpha (Timeline|Timeline PlayFromStart)
    (:Update
      (Transformation|SetRelativeScale3D (Variables|Collision|GetCapsuleComponent) (Math|Vector|Lerp(Vector) _basescale (* _basescale (Variables|Default|GetJumpSqueezeFactor)) _alpha)))))

(event Custom|RPC_FireProjectile)

(event Custom|RotateGun
  ;[1 1 1] Rotate Gun
  (Transformation|SetRelativeRotation (Variables|Default|GetScene) (Math|Rotator|MakeRotfromX (Math|Vector|ProjectVectorontoPlane (.WorldDirection (Game|Player|ConvertMouseLocationToWorldSpace (Game|GetPlayerController 0))) (Math|Vector|GetForwardVector (Variables|Default|GetCamera)))) false false))

(event Custom|RPC_Server_FireProjectile
  (CallFunction|RPCFireProjectile))

(event Custom|Flash
  (params (NumFlashes :type Integer) (FlashDuration :type Float%20%28double-precision%29) (FlashFrequency :type Float%20%28double-precision%29) (Color :type Color%20Structure))
  (bind _sprite (Variables|Default|GetSprite))
  ;[1 1 1] Flashing
  (if (< (Variables|Default|GetFlashCount) NumFlashes) :!label _label
    (Math|Integer|IncrementInt (Variables|Default|GetFlashCount)
      (:%20%20
        (Sprite|SetSpriteColor _sprite (Math|Conversions|ToLinearColor(Color) Color))
        (Utilities|FlowControl|Delay FlashDuration)
        (Sprite|SetSpriteColor _sprite "(R=1.000000,G=1.000000,B=1.000000,A=1.000000)")
        (Utilities|FlowControl|Delay FlashFrequency)
        (goto _label)))
    (else
      (Variables|Default|SetFlashCount 0))))

(event Input|EnhancedActionEvents|EnhancedInputActionIA_Jump
  (params (ActionValue :type Boolean) (ElapsedSeconds :type Float%20%28double-precision%29) (TriggeredSeconds :type Float%20%28double-precision%29) (InputAction :type Input%20Action%20Object%20Reference :default "/Game/ThirdPerson/Input/Actions/IA_Jump.IA_Jump"))
  (bind _sprite (Variables|Default|GetSprite))
  ;[1 1 1] Jump Controller
  (:Triggered
    (Character|Jump)
    (Components|Timeline|SetLooping _sprite false)
    (Sprite|SetFlipbook _sprite "/Game/2DCharacterSprites/Jump.Jump")
    (if (AI|Components|NavMovement|IsMovingonGround (Variables|Character|GetCharacterMovement))
      (CallFunction|JumpSqueeze)))
  (:Completed
    (Character|StopJumping)))

(event Input|EnhancedActionEvents|EnhancedInputActionIA_Move
  (params (ActionValue :type Vector%202D%20Structure) (ElapsedSeconds :type Float%20%28double-precision%29) (TriggeredSeconds :type Float%20%28double-precision%29) (InputAction :type Input%20Action%20Object%20Reference :default "/Game/ThirdPerson/Input/Actions/IA_Move.IA_Move"))
  ;[1 1 1] Horizontal Movement
  (:Triggered
    (Pawn|Input|AddMovementInput "1.000000,0.000000,0.000000" (.x ActionValue) false)))

(event Collision|EventHit
  (params (MyComp :type Primitive%20Component%20Object%20Reference) (Other :type Actor%20Object%20Reference) (OtherComp :type Primitive%20Component%20Object%20Reference) (bSelfMoved :type Boolean) (HitLocation :type Vector :default "0, 0, 0") (HitNormal :type Vector :default "0, 0, 0") (NormalImpulse :type Vector :default "0, 0, 0") (Hit :type Hit%20Result%20Structure%20%28by%20ref%29))
  (bind _returnvalue (Game|GetPlayerController 0))
  ;[1 1 1] GetHit
  (if (Actor|ActorHasTag Other "Bullet")
    (Character|LaunchCharacter (+ (* HitNormal "1000.000000,1000.000000,1000.000000") "0.000000,0.000000,700.000000") false false)
    (CallFunction|Flash 3 0.1 0.1 (Math|Color|MakeColor 0 0 255 255))
    (Input|SetIgnoreMoveInput _returnvalue true)
    (Utilities|FlowControl|Delay (Variables|Default|GetHitStunDurration))
    (Input|SetIgnoreMoveInput _returnvalue false)
    (Input|ResetIgnoreMoveInput _returnvalue)))

(event EventBeginPlay
  ;[0.05098 0.05098 0.05098] Start
  (CallFunction|SetupInputMapping)
  (Variables|Default|SetBaseScale (Variables|/Script/Engine.SceneComponent|GetRelativeScale3D (Variables|Collision|GetCapsuleComponent)))
  (Variables|/Script/Engine.PlayerController|SetbShowMouseCursor (Game|GetPlayerController 0) true))

(event EventTick
  (params (DeltaSeconds :type Float%20%28single-precision%29))
  ;[1 1 1] Update
  (if (not (Variables|Default|GetAnimationOverride))
    (CallFunction|UpdateGroundAnimation)
    (CallFunction|UpdateSpriteFlipping)
    (CallFunction|RotateGun)))

(event EventOnLanded
  (params (Hit :type Hit%20Result%20Structure%20%28by%20ref%29))
  (bind _sprite (Variables|Default|GetSprite))
  ;[1 1 1] Landing
  (Components|Timeline|SetLooping _sprite true)
  (Audio|Components|Audio|Play _sprite)
  (CallFunction|LandSquish))

(event Input|MouseEvents|RightMouseButton
  (params (Key :type Key%20Structure :default "None"))
  (bind _sprite (Variables|Default|GetSprite))
  (:Pressed
    (Variables|Default|SetAnimationOverride true)
    (Components|Timeline|SetLooping _sprite false)
    (Sprite|SetFlipbook _sprite "/Game/2DCharacterSprites/YH_Cowboy_HSlashF1.YH_Cowboy_HSlashF1")
    (bind _outactors (Collision|ComponentOverlapActors (Variables|Default|GetChargeBackRange) (Transformation|GetWorldTransform (Variables|Default|GetChargeBackRange)) (Utilities|Array|MakeArray "ObjectTypeQuery8") "/Game/Blueprints/BP_BaseProjectile.BP_BaseProjectile_C"))
    (for _array_element _outactors
      (Transformation|SetActorRotation _array_element (Variables|/Script/Engine.SceneComponent|GetRelativeRotation (Variables|Default|GetScene)))
      (CallFunction|Flash 1 0.1 0.0 (Math|Color|MakeColor 0 255 0 255)))))

(event Input|MouseEvents|LeftMouseButton
  (params (Key :type Key%20Structure :default "None"))
  (bind _bulletspawn (Variables|Default|GetBulletSpawn))
  (bind _returnvalue (Transformation|GetWorldTransform _bulletspawn))
  (bind (_location _rotation) (Math|Transform|BreakTransform _returnvalue))
  ;[1 1 1] Shooting
  (:Pressed
    (bind _returnvalue_2 (Game|SpawnActorfromClass "/Game/Blueprints/BP_BaseProjectile.BP_BaseProjectile_C" (Math|Transform|MakeTransform _location _rotation) "AdjustIfPossibleButAlwaysSpawn" 0 self))
    (Variables|/Script/Engine.MovementComponent|SetVelocity (Variables|/Game/Blueprints/BP_BaseProjectile.BP_BaseProjectile_C|GetProjectileMovement _returnvalue_2) (+ (Variables|/Script/Engine.MovementComponent|GetVelocity (Variables|/Game/Blueprints/BP_BaseProjectile.BP_BaseProjectile_C|GetProjectileMovement _returnvalue_2)) (Math|Vector|ProjectVectorontoVector (Pawn|Components|CharacterMovement|GetLastUpdateVelocity (Variables|Character|GetCharacterMovement)) (Variables|/Script/Engine.MovementComponent|GetVelocity (Variables|/Game/Blueprints/BP_BaseProjectile.BP_BaseProjectile_C|GetProjectileMovement _returnvalue_2)))))))

(event Input|KeyboardEvents|C
  (params (Key :type Key%20Structure :default "None"))
  (bind _sprite (Variables|Default|GetSprite))
  (:Pressed
    (Variables|Default|SetAnimationOverride true)
    (Components|Timeline|SetLooping _sprite false)
    (Sprite|SetFlipbook _sprite "/Game/2DCharacterSprites/YH_Cowboy_HSlashF1.YH_Cowboy_HSlashF1")
    (bind _outactors (Collision|ComponentOverlapActors (Variables|Default|GetChargeBackRange) (Transformation|GetWorldTransform (Variables|Default|GetChargeBackRange)) (Utilities|Array|MakeArray "ObjectTypeQuery8") "/Game/Blueprints/BP_BaseProjectile.BP_BaseProjectile_C"))
    (for _array_element _outactors
      (Transformation|SetActorRotation _array_element (Variables|/Script/Engine.SceneComponent|GetRelativeRotation (Variables|Default|GetScene)))
      (CallFunction|Flash 1 0.1 0.0 (Math|Color|MakeColor 0 255 0 255)))))

(fn ConstructionScript)

(fn SetupInputMapping
  (bind _asplayer_controller (Utilities|Casting|CastToPlayerController (Pawn|GetController)))
  (Utilities|IsValid (PlayerController|LocalPlayerSubsystems|GetEnhancedInputLocalPlayerSubsystem _asplayer_controller)
    (:Is%20Valid
      (Input|AddMappingContext (PlayerController|LocalPlayerSubsystems|GetEnhancedInputLocalPlayerSubsystem _asplayer_controller) "/Game/ThirdPerson/Input/IMC_Default.IMC_Default" 0 "(bIgnoreAllPressedKeysUntilRelease=True,bForceImmediately=False)"))))